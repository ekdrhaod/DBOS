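; Frosty is a playable character Blueprint with a ranged attack, a W-key skill and its own damage and death handling.
; Attack fires a projectile and the skill spawns effect and skill actors with sound, each gated by a boolean-and-Delay cooldown.
; Hits from projectiles or skill_b_w subtract HP through DoOnce gates while briefly toggling capsule physics; projectiles also launch the character along the hit normal.
; Exactly zero HP triggers destruction and spawns a Death actor.
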(event Custom|공격
  (bind _capsulecomponent (Variables|Default|GetCapsuleComponent))
  (bind _returnvalue (Transformation|GetWorldRotation _capsulecomponent))
  ;[1 1 1] 공격 나가기
  (if (not (Variables|Default|Getshoot))
    (Variables|Default|Setshoot true)
    (Game|SpawnActorfromClass "/Game/Blueprints/Characters/charac_dbos/FirstPersonProjectile.FirstPersonProjectile_C" (Math|Transform|MakeTransform (+ (Transformation|GetWorldLocation (Variables|Default|Getattack)) (Math|Vector|RotateVector (Variables|Default|GetGun%20Offset) _returnvalue)) _returnvalue) "AdjustIfPossibleButDontSpawnIfColliding" 0 0)
    (Audio|PlaySoundatLocation 0 (Transformation|GetActorLocation))
    (Utilities|FlowControl|Delay 2.0)
    (Variables|Default|Setshoot false)))

(event Custom|스킬
  (bind _capsulecomponent (Variables|Default|GetCapsuleComponent))
  (bind _returnvalue (Transformation|GetWorldRotation _capsulecomponent))
  ;[1 1 1] 스킬
  (if (not (Variables|Default|Getskill_x))
    (Game|SpawnActorfromClass "/Game/Blueprints/Characters/charac_dbos/spawn_frosty.spawn_frosty_C" (Math|Conversions|ToTransform(Vector) (Transformation|GetWorldLocation _capsulecomponent)) "Undefined" 0 0)
    (Components|Animation|PlayAnimation (Variables|Character|GetMesh) "/Game/Blueprints/Characters/charac_dbos/호구/anim/Whiteclown_N_Hallin_mixamo_com.Whiteclown_N_Hallin_mixamo_com" false)
    (Variables|Default|Setskill_x true)
    (Game|SpawnActorfromClass "/Game/Blueprints/Characters/charac_dbos/skill_x_w.skill_x_w_C" (Math|Transform|MakeTransform (+ (Transformation|GetWorldLocation (Variables|Default|Getattack)) (Math|Vector|RotateVector "0.000000, 0, 0" _returnvalue)) _returnvalue) "AdjustIfPossibleButDontSpawnIfColliding" 0 0)
    (Audio|PlaySoundatLocation 0 (Transformation|GetActorLocation))
    (Components|Animation|SetAnimationMode (Variables|Character|GetMesh) "AnimationBlueprint")
    (Utilities|FlowControl|Delay 5.0)
    (Variables|Default|Setskill_x false)))

(event Collision|EventHit
  (params (MyComp :type Primitive%20Component%20Object%20Reference) (Other :type Actor%20Object%20Reference) (OtherComp :type Primitive%20Component%20Object%20Reference) (bSelfMoved :type Boolean) (HitLocation :type Vector :default "0, 0, 0") (HitNormal :type Vector) (NormalImpulse :type Vector :default "0, 0, 0") (Hit :type Hit%20Result%20Structure%20%28by%20ref%29))
  (bind _returnvalue (* HitNormal 3e+03))
  (bind _mesh (Variables|Character|GetMesh))
  (bind _mesh_2 (Variables|Character|GetMesh))
  (bind (_x _y) (Math|Vector|BreakVector _returnvalue))
  (Utilities|FlowControl|Sequence
    (:then_0
      ;[1 1 1] 코멘트
      (bind _asfirst_person_projectile (Utilities|Casting|CastToFirstPersonProjectile Other))
      (Utilities|FlowControl|DoOnce false :!label _label
        (:Completed
          (Utilities|FlowControl|Sequence
            (:then_0
              (Physics|SetSimulatePhysics (Variables|Default|GetCapsuleComponent) true)
              (bind _output_get (Variables|Default|Setcur%20HP (- (Variables|Default|Getcur%20HP) 2e+01)))
              (if (== _output_get 0.0)
                (Development|PrintString "dead")
                (Components|Animation|PlayAnimation _mesh "/Game/Blueprints/Characters/charac_dbos/호구/Whiteclown_N_Hallin_Anim_mixamo_com.Whiteclown_N_Hallin_Anim_mixamo_com" false)
                (Actor|DestroyActor)
                (Game|SpawnActorfromClass "/Game/Blueprints/Characters/charac_dbos/death.death_C" (Math|Conversions|ToTransform(Vector) (Transformation|GetWorldLocation _mesh)) "Undefined" 0 0)
                (else
                  (Development|PrintString "live")
                  (Utilities|FlowControl|Delay 0.0)
                  (Physics|SetSimulatePhysics (Variables|Default|GetCapsuleComponent) false)
                  (goto _label Reset))))
            (:then_1
              (Character|LaunchCharacter (Math|Vector|MakeVector _x _y 0.0) false false))))))
    (:then_1
      (bind _asskill_b_w (Utilities|Casting|CastToskill_b_w Other))
      (Utilities|FlowControl|DoOnce false :!label _label_2
        (:Completed
          (Physics|SetSimulatePhysics (Variables|Default|GetCapsuleComponent) true)
          (bind _output_get_2 (Variables|Default|Setcur%20HP (- (Variables|Default|Getcur%20HP) 3e+01)))
          (if (== _output_get_2 0.0)
            (Development|PrintString "dead")
            (Components|Animation|PlayAnimation _mesh_2 "/Game/Blueprints/Characters/charac_dbos/법사/anim/Standing_React_Death_Backward.Standing_React_Death_Backward" false)
            (Game|SpawnActorfromClass "/Game/Blueprints/Characters/charac_dbos/death.death_C" (Math|Conversions|ToTransform(Vector) (Transformation|GetWorldLocation _mesh_2)) "Undefined" 0 0)
            (Actor|DestroyActor)
            (else
              (Development|PrintString "live")
              (Utilities|FlowControl|Delay 0.0)
              (Physics|SetSimulatePhysics (Variables|Default|GetCapsuleComponent) false)
              (goto _label_2 Reset))))))))

(event Input|ActionEvents|InputActionattack
  (params (Key :type Key%20Structure :default "AnyKey"))
  (:Pressed
    (CallFunction|공격)))

(event Input|KeyboardEvents|W
  (params (Key :type Key%20Structure :default "AnyKey"))
  (:Pressed
    (CallFunction|스킬)))

(fn ConstructionScript
  (|CallParentFunction))